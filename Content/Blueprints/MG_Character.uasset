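; Player character for a side-scrolling 2D game that runs automatically along X and moves vertically toward the clicked point.
; MouseClick stores the hit location under the cursor with Y zeroed, printing it to the log for debugging.
; Each Tick teleport-steps X by MoveSpeedX without sweep and sets the run flipbook.
; CharacterMove then steps MovePosZ toward the clicked Z by MoveSpeedZ, applied on the following Tick.
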(event EventBeginPlay
  (Utilities|FlowControl|Sequence
    (:then_0
      ;[1 1 1] speichert aktuelle position von charakter
      (Variables|Default|SetcharakterPos (Transformation|GetActorLocation)))))

(event EventTick
  (params (DeltaSeconds :type Float%20%28single-precision%29))
  (Utilities|FlowControl|Sequence
    (:then_0
      ;[1 1 1] bewegt charakter in x-richtung
      (Variables|Default|SetcharakterPos (Math|Vector|MakeVector (+ (.X (Math|Vector|BreakVector (Variables|Default|GetcharakterPos))) (Variables|Default|GetmoveSpeedX)) 0.0 (Variables|Default|GetmovePosZ)))
      (Transformation|SetActorLocation (Variables|Default|GetcharakterPos) false false)
      (Sprite|SetFlipbook (Variables|Default|GetSprite) "/Game/Sprites/Character/Run/character_run.character_run"))
    (:then_1
      (CallFunction|CharacterMove) ; funktion charakter bewegung durch mausklick in z-richtung +-
    )))

(event Input|ActionEvents|InputActionMouseClick
  (params (Key :type Key%20Structure))
  (bind _returnvalue (Game|GetPlayerController 0))
  (bind _hitresult (Game|Player|GetHitResultUnderCursorbyChannel _returnvalue "TraceTypeQuery1" true))
  (bind _location (Collision|BreakHitResult _hitresult))
  (bind (_x _y _z) (Math|Vector|BreakVector _location))
  (:Pressed
    ;[1 1 1] aktuelle maus-position abfragen/speichern
    (Variables|Default|SetcurrentMousePos (Math|Vector|MakeVector _x 0.0 _z))
    (Utilities|FlowControl|DoN 1 :!label _label
      (:Exit
        ;[1 1 1] debug / print aktuelle maus pos
        (Development|PrintString (Utilities|String|ToString(Vector) (Variables|Default|GetcurrentMousePos)) false))))
  (:Released
    (goto _label Reset)))

(fn ConstructionScript)

(fn CharacterMove
  (bind _currentmousepos (Variables|Default|GetcurrentMousePos))
  (bind _charakterpos (Variables|Default|GetcharakterPos))
  (bind _movespeedz (Variables|Default|GetmoveSpeedZ))
  (bind _z (Math|Vector|BreakVector _currentmousepos))
  (bind _z_2 (Math|Vector|BreakVector _charakterpos))
  (bind _returnvalue (- _z_2 _movespeedz))
  (bind _returnvalue_2 (+ _z_2 _movespeedz))
  (if (<= _returnvalue_2 _z)
    (Variables|Default|SetmovePosZ _returnvalue_2)
    (elif (>= _returnvalue _z)
      (Variables|Default|SetmovePosZ _returnvalue))))