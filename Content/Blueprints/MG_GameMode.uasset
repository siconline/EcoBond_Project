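; MG_GameMode is a game mode that runs a countdown timer and ends play when time runs out.
; Tick feeds a one-second Delay, so the Seconds counter drops about once per second and rolls over into Minutes below zero.
; When both counters reach zero, it prints a time-out message and pauses the game, with no further game-over handling.
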(event EventTick
  (params (DeltaSeconds :type Float%20%28single-precision%29))
  ;[1 1 1] timer für gameover wenn zeit abgelaufen ist
  (Utilities|FlowControl|Delay 1.0)
  (Variables|Default|Setseconds (- (Variables|Default|Getseconds) 1))
  (if (< (Variables|Default|Getseconds) 0)
    (Variables|Default|Setminutes (- (Variables|Default|Getminutes) 1))
    (Variables|Default|Setseconds 59))
  (if (== (Variables|Default|Getseconds) 0)
    (if (== (Variables|Default|Getminutes) 0)
      (Development|PrintString "time out")
      (Game|SetGamePaused true))))

(fn ConstructionScript)